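; Timed Hardpoint capture zone for Mordhau that awards team and player score while only one team occupies it.
; Server box overlaps maintain per-team character lists, whose RepNotify counts drive looping score timers, paused when contested or empty, and the zone material.
; Activation announces the point and starts a lifetime timer that deactivates it on expiry.
; The construction script sizes mesh and box; a widget shows team counts and color.
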(event OnComponentBeginOverlap(Box)
  (params (OverlappedComponent :type Primitive%20Component%20Object%20Reference) (OtherActor :type Actor%20Object%20Reference) (OtherComp :type Primitive%20Component%20Object%20Reference) (OtherBodyIndex :type Integer) (bFromSweep :type Boolean) (SweepResult :type Hit%20Result%20Structure%20%28by%20ref%29))
  ;[1 0 0.1339 1 80] Entering and exiting the point
  (Networking|SwitchHasAuthority
    (:Authority
      (Update|ProcessCharacter OtherActor true))
    (:Remote
      (if (Variables|Default|GetShouldPlaySound)
        (Audio|PlaySound2D "/Game/Mordhau/Audio/Raw/Misc/Other/Sticks1.Sticks1" 1.0 1.0 0.0 0 0)))))

(event OnComponentEndOverlap(Box)
  (params (OverlappedComponent :type Primitive%20Component%20Object%20Reference) (OtherActor :type Actor%20Object%20Reference) (OtherComp :type Primitive%20Component%20Object%20Reference) (OtherBodyIndex :type Integer))
  ;[1 0 0.1339 1 80] Entering and exiting the point
  (Networking|SwitchHasAuthority
    (:Authority
      (Update|ProcessCharacter OtherActor false))
    (:Remote
      (if (Variables|Default|GetShouldPlaySound)
        (Audio|PlaySound2D "/Game/Mordhau/Audio/Raw/Misc/Other/Sticks2.Sticks2" 1.0 1.0 0.0 0 0)))))

(event Custom|AddScoreTeam0
  (bind _scorebonus (Variables|Hardpoint|GetscoreBonus))
  (bind _returnvalue (+ 1.0 _scorebonus))
  ;[1 0.6349 0 1 80] Scoring
  (Networking|SwitchHasAuthority
    (:Authority
      ;;[1 1 1] Pause the other team's addScoreTimer (so only 1 team gets score)
      (Utilities|Time|PauseTimerbyHandle (Variables|Private|GetAddScoreTeam1Timer))
      ;;[1 1 1] Add Team Score
      (Class|MordhauGameMode|AddTeamScore (Variables|Private|GetHardpoint%20Gamemode) 0 _returnvalue)
      ;;[1 1 1] Loop Through all players on point
      (for _array_element (Variables|Private|Getteam0)
        ;;[1 1 1] Award PLAYER SCORE to all players on point
        (bind _asmordhau_player_controller (Utilities|Casting|CastToMordhauPlayerController (Pawn|GetController _array_element)))
        (Class|MordhauPlayerController|GiveClientScoreBP _asmordhau_player_controller "Objective" (Math|Float|Truncate _returnvalue))))))

(event Custom|AddScoreTeam1
  (bind _scorebonus (Variables|Hardpoint|GetscoreBonus))
  (bind _returnvalue (+ 1.0 _scorebonus))
  ;[1 0.6349 0 1 80] Scoring
  (Networking|SwitchHasAuthority
    (:Authority
      ;;[1 1 1] Pause the other team's addScoreTimer (so only 1 team gets score)
      (Utilities|Time|PauseTimerbyHandle (Variables|Private|GetAddScoreTeam0Timer))
      ;;[1 1 1] Add Team Score
      (Class|MordhauGameMode|AddTeamScore (Variables|Private|GetHardpoint%20Gamemode) 1 _returnvalue)
      ;;[1 1 1] Loop Through all players on point
      (for _array_element (Variables|Private|Getteam1)
        ;;[1 1 1] Award PLAYER SCORE to all players on point
        (bind _asmordhau_player_controller (Utilities|Casting|CastToMordhauPlayerController (Pawn|GetController _array_element)))
        (Class|MordhauPlayerController|GiveClientScoreBP _asmordhau_player_controller "Objective" (Math|Float|Truncate _returnvalue))))))

(event Custom|ServerSwitchPoint
  ;[0.1194 0.5968 1 1 80] Switch to next Hardpoint
  ;;[1 0 0 1 10] Server Call
  (CallFunction|ClientSwitchPoint))

(event Custom|ServerSetActive
  ;[0.2603 1 0 1 80] Point is On/Off
  ;;[1 0 0 1 10] Server Call
  (CallFunction|ClientSetActive))

(event Custom|ClientSwitchPoint
  ;[0.1194 0.5968 1 1 80] Switch to next Hardpoint
  (Audio|PlaySound2D "/Game/Mordhau/Audio/Raw/Misc/Other/Bell.Bell" 1.0 1.0 0.0 0 0)
  (CallFunction|ServerSetInactive))

(event Custom|Server%20UpdateUIPlayerCount
  (CallFunction|ClientUpdateUIPlayerCount))

(event Custom|ClientUI
  ;[1 1 1 1 80] Point UI Icon Init
  (Networking|CanExecuteCosmeticEvents
    (:True
      (bind _asui_point_icon (Utilities|Casting|CastToUI_PointIcon (UserInterface|GetUserWidgetObject (Variables|Default|GetPointUI))))
      (Variables|/Game/Mordhau/Maps/Mordhau-Hardpoint/Assets/BPS/UI_PointIcon.UI_PointIcon_C|SetHardpoint%20Parent _asui_point_icon self)
      (Appearance|SetBrushfromTexture (Variables|/Game/Mordhau/Maps/Mordhau-Hardpoint/Assets/BPS/UI_PointIcon.UI_PointIcon_C|GetIcon _asui_point_icon) (Variables|Color|GetIcon) true)
      (UI|ToggleWidget (Variables|HardpointSystem|GetActive)))))

(event Custom|ClientUpdate
  (bind _scoreinterval (Variables|Hardpoint|GetscoreInterval))
  (bind _team0 (Variables|Private|Getteam0))
  (bind _returnvalue (Utilities|Array|Length _team0))
  (bind _returnvalue_2 (!= _returnvalue 0))
  (if (Variables|HardpointSystem|GetActive)
    (Networking|SwitchHasAuthority
      (:Authority
        (if (Class|KismetMathLibrary|XORBoolean _returnvalue_2 (!= (Utilities|Array|Length (Variables|Private|Getteam1)) 0))
          (if _returnvalue_2
            (if (Class|KismetSystemLibrary|TimerExistsHandle (Variables|Private|GetAddScoreTeam0Timer))
              (if (Class|KismetSystemLibrary|IsTimerPausedHandle (Variables|Private|GetAddScoreTeam0Timer))
                (Utilities|Time|UnpauseTimerbyHandle (Variables|Private|GetAddScoreTeam0Timer))
                (Debug|DebugPrint "Resumed Team0 Score Timer" "(R=0.000000,G=1.000000,B=0.043137,A=1.000000)"))
              (else
                (bind _returnvalue_3 (Utilities|Time|SetTimerbyEvent (EventDispatchers|CreateEvent :!event Custom|AddScoreTeam0) _scoreinterval true))
                (Variables|Private|SetAddScoreTeam0Timer _returnvalue_3)
                (Debug|DebugPrint "Created New Team0 Score Timer" "(R=0.000000,G=1.000000,B=0.043137,A=1.000000)")))
            (elif (Class|KismetSystemLibrary|TimerExistsHandle (Variables|Private|GetAddScoreTeam1Timer))
              (if (Class|KismetSystemLibrary|IsTimerPausedHandle (Variables|Private|GetAddScoreTeam1Timer))
                (Utilities|Time|UnpauseTimerbyHandle (Variables|Private|GetAddScoreTeam1Timer))
                (Debug|DebugPrint "Resumed Team1 Score Timer" "(R=0.000000,G=1.000000,B=0.043137,A=1.000000)"))
              (else
                (bind _returnvalue_4 (Utilities|Time|SetTimerbyEvent (EventDispatchers|CreateEvent :!event Custom|AddScoreTeam1) _scoreinterval true))
                (Variables|Private|SetAddScoreTeam1Timer _returnvalue_4)
                (Debug|DebugPrint "Created New Team1 Score Timer" "(R=0.000000,G=1.000000,B=0.043137,A=1.000000)"))))
          (else
            (Update|PauseAllTimers true)))))))

(event Custom|ServerUpdate
  (CallFunction|ClientUpdate))

(event Custom|ServerUI
  ;[1 1 1 1 80] Point UI Icon Init
  (CallFunction|ClientUI))

(event Custom|ClientSetLocation
  (bind _mordhauscene (Variables|Default|GetMordhauScene))
  (bind _returnvalue (Transformation|GetWorldLocation _mordhauscene))
  (bind _returnvalue_2 (Transformation|GetWorldRotation _mordhauscene))
  (bind _returnvalue_3 (Math|Vector|GetUpVector _returnvalue_2))
  (bind (_x _y _z) (Math|Vector|BreakVector _returnvalue_3))
  ;[0 1 0.9308] Raytracing. Only used/useful for blindly making maps (ie, you don't know where floor is? Ray trace on BeginPlay() )
  (bind _outhit (Collision|LineTraceByChannel _returnvalue (+ _returnvalue (* (Math|Vector|MakeVector _x _y (* _z -1.0)) 1.5e+03)) "TraceTypeQuery1" false 0 "ForOneFrame"))
  (Transformation|SetWorldLocation (Variables|Default|GetMordhauScene) (.Location (Collision|BreakHitResult _outhit)) false true))

(event Custom|Server%20Set%20Location
  ;[0 1 0.9308] Raytracing. Only used/useful for blindly making maps (ie, you don't know where floor is? Ray trace on BeginPlay() )
)

(event Custom|ServerAddScoreTeam0
  ;[1 0.6349 0 1 80] Scoring
  ;;[1 0 0] Server Runs this then -->
  (CallFunction|AddScoreTeam0))

(event Custom|ServerAddScoreTeam1
  ;[1 0.6349 0 1 80] Scoring
  ;;[1 0 0] Server Runs this then -->
  (CallFunction|AddScoreTeam1))

(event Custom|ClientSetInactive
  ;[0.2603 1 0 1 80] Point is On/Off
  (Update|SetInactive)
  (Utilities|Array|Clear (Variables|Private|Getteam0))
  (Utilities|Array|Clear (Variables|Private|Getteam1))
  (CallFunction|ServerUpdate))

(event Custom|ClientSetActive
  ;[0.2603 1 0 1 80] Point is On/Off
  (Update|SetActive)
  (bind _returnvalue (Utilities|Time|SetTimerbyEvent (delegate Custom|ClientSwitchPoint) (Variables|Hardpoint|GetpointDuration)))
  (Variables|Private|SetLifeHandle _returnvalue)
  (bind _returnvalue_2 (Utilities|Time|SetTimerbyEvent (delegate Custom|Server%20UpdateUIPlayerCount) 0.2 true))
  (Variables|Private|SetPercentTimer _returnvalue_2)
  (UI|MakeAnnouncement "New Hardpoint!" 4.0)
  (CallFunction|ServerUpdate))

(event Custom|ClientUpdateColor
  ;[0.766 1 0.2114 1 80] Update Hardpoint Color
  (Color|SetPointColor)
  (UI|SetPointIconColor))

(event Custom|ServerSetInactive
  ;[0.2603 1 0 1 80] Point is On/Off
  ;;[1 0 0 1 10] Server Call
  (CallFunction|ClientSetInactive))

(event Custom|ServerUpdateColor
  ;[0.766 1 0.2114 1 80] Update Hardpoint Color
  ;;[1 0 0 1 10] Server Call
  (CallFunction|ClientUpdateColor))

(event Custom|Client%20UpdateUIPlayerCount
  (bind _lifehandle (Variables|Private|GetLifeHandle))
  (bind _pointduration (Variables|Hardpoint|GetpointDuration))
  (bind _returnvalue (Utilities|Time|GetTimerRemainingTimebyHandle _lifehandle))
  (bind _returnvalue_2 (/ _returnvalue _pointduration))
  (UI|UpdatePointIconData (Utilities|Array|Length (Variables|Private|Getteam0)) (Utilities|Array|Length (Variables|Private|Getteam1)) _returnvalue_2)
  (UI|SetPointIconColor)
  (Networking|SwitchHasAuthority
    (:Authority
      (Variables|Default|SetPointTimeRemaining _returnvalue_2))))

(event EventBeginPlay
  ;[0 1 0.9624 1 80] Init
  (bind _asmordhau_game_mode (Utilities|Casting|CastToMordhauGameMode (Game|GetGameMode))
    (:then
      (Variables|Private|SetHardpoint%20Gamemode _asmordhau_game_mode))
    (:CastFailed
      _))
  (CallFunction|ClientUI))

(event Input|KeyboardEvents|F5
  (params (Key :type Key%20Structure :default "None"))
  ;[1 1 1] Add this to the level BP to enable sound for when someone steps on point. Should be client sided, tho untested
  (:Released
    (bind _outactors (Actor|GetAllActorsOfClass "BP_Hardpoint_C"))
    (for _array_element _outactors
      (Variables|BP_Hardpoint_C|SetShouldPlaySound _array_element (not (Variables|BP_Hardpoint_C|GetShouldPlaySound _array_element))))))

(fn ConstructionScript
  (Variables|Scale|SetX (* (Variables|Scale|GetX) "1.000000, 0,0.000000"))
  (Variables|Scale|SetY (* (Variables|Scale|GetY) "0,1.000000, 0"))
  (Variables|Scale|SetZ (* (Variables|Scale|GetZ) "0,0.000000,1.000000"))
  (Construction|UpdateSize)
  (CallFunction|ServerUpdate)
  (CallFunction|ServerUpdateColor)
  (CallFunction|ServerUI)
  (if (Variables|HardpointSystem|GetActive)
    (Variables|RepNotify|SetCurrentMat (Variables|Color|GetActive%20Mat))))

(fn UpdateSize
  (bind _x (Variables|Scale|GetX))
  (bind _y (Variables|Scale|GetY))
  (bind _z (Variables|Scale|GetZ))
  (bind _box (Variables|Default|GetBox))
  (bind _x_2 (Math|Vector|BreakVector _x))
  (bind _z_2 (Math|Vector|BreakVector _z))
  (bind _returnvalue (Components|Box|GetUnscaledBoxExtent _box))
  (bind _y_2 (Math|Vector|BreakVector _y))
  (bind _relativelocation (Variables|/Script/Engine.SceneComponent|GetRelativeLocation _box))
  (bind (_x_3 _y_3) (Math|Vector|BreakVector _returnvalue))
  (bind (_x_4 _y_4) (Math|Vector|BreakVector _relativelocation))
  (bind _returnvalue_2 (/ _x_2 4e+02))
  (bind _returnvalue_3 (/ _y_2 4e+02))
  (bind _returnvalue_4 (* _returnvalue_2 8.0))
  (bind _returnvalue_5 (* _returnvalue_3 8.0))
  (Transformation|SetWorldScale3D (Variables|Default|GetStaticMesh) (Math|Vector|MakeVector _returnvalue_4 _returnvalue_5 0.1))
  (Transformation|SetWorldScale3D (Variables|Default|GetBox) (Math|Vector|MakeVector _returnvalue_4 _returnvalue_5 4.0))
  (Components|Box|SetBoxExtent _box (Math|Vector|MakeVector _x_3 _y_3 (* (/ _z_2 1e+02) 12.5)) true)
  (Transformation|SetRelativeLocation _box (Math|Vector|MakeVector _x_4 _y_4 (/ _z_2 2.0)) false true))

(fn ProcessCharacter
  (params (Actor :type Object%20Object%20Reference%20%28by%20ref%29) (ShouldAdd :type Boolean))
  (bind _lifehandle (Variables|Private|GetLifeHandle))
  (bind _team1 (Variables|Private|Getteam1))
  (bind _team0 (Variables|Private|Getteam0))
  (bind _returnvalue (Class|KismetSystemLibrary|TimerExistsHandle _lifehandle))
  (Networking|SwitchHasAuthority
    (:Authority
      (Development|PrintString "Server Processesing Character" true true "(R=1.000000,G=0.000000,B=0.079762,A=1.000000)"))
    (:Remote
      (Development|PrintString "Client Processesing Character" true true "(R=0.000000,G=1.000000,B=0.108814,A=1.000000)")))
  (bind _asmordhau_character (Utilities|Casting|CastToMordhauCharacter Actor))
  (bind _output_get (LocalVariables|SetCharacter _asmordhau_character))
  (if (== (Variables|/Script/Mordhau.AdvancedCharacter|GetTeam _output_get) 0)
    (if ShouldAdd
      (Utilities|Array|AddUnique _team0 (LocalVariables|GetCharacter))
      (else
        (Utilities|Array|RemoveItem _team0 (LocalVariables|GetCharacter))))
    (if _returnvalue
      (Variables|RepNotify|SetTeam0PlayersOnPoint (Utilities|Array|Length _team0)))
    (else
      (if ShouldAdd
        (Utilities|Array|AddUnique _team1 (LocalVariables|GetCharacter))
        (else
          (Utilities|Array|RemoveItem _team1 (LocalVariables|GetCharacter))))
      (if _returnvalue
        (Variables|RepNotify|SetTeam1PlayersOnPoint (Utilities|Array|Length _team1))))))

(fn ToggleWidget
  (params (State :type Boolean))
  (bind _pointui (Variables|Default|GetPointUI))
  (bind _returnvalue (UserInterface|GetUserWidgetObject _pointui))
  (Networking|CanExecuteCosmeticEvents
    (:True
      (Utilities|IsValid _pointui
        (:Is%20Valid
          (if State
            (Widget|SetVisibility _returnvalue "HitTestInvisible")
            (else
              (Widget|SetVisibility _returnvalue "Collapsed"))))))))

(fn MakeAnnouncement
  (params (Message :type Text) (Duration :type Float%20%28single-precision%29))
  (bind _asbp_mordhau_hud (Utilities|Casting|CastToBP_MordhauHUD (Class|MordhauUtilityLibrary|GetMordhauHUD (Game|GetPlayerCharacter 0))))
  (Default|ShowAnnouncement _asbp_mordhau_hud Message (Utilities|Text|FormatText "Lifespan: {a}s" (Utilities|Text|ToText(Float) (Variables|Hardpoint|GetpointDuration) "HalfToEven")) Duration "NewEnumerator0"))

(fn SetPointIconColor
  (bind _currentmat (Variables|RepNotify|GetCurrentMat))
  (bind _asui_point_icon (Utilities|Casting|CastToUI_PointIcon (UserInterface|GetUserWidgetObject (Variables|Default|GetPointUI))))
  (if (== _currentmat (Variables|Color|GetInactive%20Mat))
    (bind _result (Color|GetColor "NewEnumerator0"))
    (Class|Image|SetBrushTintColor (Variables|/Game/Mordhau/Maps/Mordhau-Hardpoint/Assets/BPS/UI_PointIcon.UI_PointIcon_C|GetIcon _asui_point_icon) _result)
    (elif (== _currentmat (.Value (Utilities|Map|Find (Variables|Color|GetTeamColors) "NewEnumerator0")))
      (bind _result_2 (Color|GetColor "NewEnumerator3"))
      (Class|Image|SetBrushTintColor (Variables|/Game/Mordhau/Maps/Mordhau-Hardpoint/Assets/BPS/UI_PointIcon.UI_PointIcon_C|GetIcon _asui_point_icon) _result_2)
      (elif (== _currentmat (.Value (Utilities|Map|Find (Variables|Color|GetTeamColors) "NewEnumerator1")))
        (bind _result_3 (Color|GetColor "NewEnumerator2"))
        (Class|Image|SetBrushTintColor (Variables|/Game/Mordhau/Maps/Mordhau-Hardpoint/Assets/BPS/UI_PointIcon.UI_PointIcon_C|GetIcon _asui_point_icon) _result_3)
        (else
          (bind _result_4 (Color|GetColor "NewEnumerator0"))
          (Class|Image|SetBrushTintColor (Variables|/Game/Mordhau/Maps/Mordhau-Hardpoint/Assets/BPS/UI_PointIcon.UI_PointIcon_C|GetIcon _asui_point_icon) _result_4))))))

(fn PauseAllTimers
  (params (Just%20Team%20Timers :type Boolean))
  (bind _addscoreteam1timer (Variables|Private|GetAddScoreTeam1Timer))
  (bind _addscoreteam0timer (Variables|Private|GetAddScoreTeam0Timer))
  (bind _lifehandle (Variables|Private|GetLifeHandle))
  (bind _percenttimer (Variables|Private|GetPercentTimer))
  (if Just%20Team%20Timers
    _
    (else
      (if (Utilities|Time|IsTimerActivebyHandle _lifehandle)
        (Utilities|Time|PauseTimerbyHandle _lifehandle))
      (if (Utilities|Time|IsTimerActivebyHandle _percenttimer)
        (Utilities|Time|PauseTimerbyHandle _percenttimer))))
  (if (Utilities|Time|IsTimerActivebyHandle _addscoreteam0timer)
    (Utilities|Time|PauseTimerbyHandle _addscoreteam0timer))
  (if (Utilities|Time|IsTimerActivebyHandle _addscoreteam1timer)
    (Utilities|Time|PauseTimerbyHandle _addscoreteam1timer)))

(fn SetActive
  (Variables|HardpointSystem|SetActive true)
  (Variables|RepNotify|SetCurrentMat (Variables|Color|GetActive%20Mat))
  (UI|ToggleWidget true)
  (UI|SetPointIconColor))

(fn SetInactive
  (Variables|HardpointSystem|SetActive false)
  (Variables|RepNotify|SetTeam1PlayersOnPoint 0)
  (Variables|RepNotify|SetTeam0PlayersOnPoint 0)
  (Variables|RepNotify|SetCurrentMat (Variables|Color|GetInactive%20Mat))
  (UI|ToggleWidget false)
  (Update|PauseAllTimers false))

(fn GetColor
  (params (Color :type E_HardpointColors%20Enum :default "NewEnumerator0"))
  (bind _struct_colors (LocalVariables|GetSTRUCT_Colors))
  (bind (_active _inactive _redteam _blueteam) (Utilities|Struct|BreakSTRUCT_Colors _struct_colors))
  (switch Utilities|FlowControl|Switch|SwitchonE_HardpointColors Color
    (:NewEnumerator0
      (return _active))
    (:NewEnumerator1
      (return _inactive))
    (:NewEnumerator2
      (return _redteam))
    (:NewEnumerator3
      (return _blueteam))))

(fn DebugPrint
  (params (Msg :type String) (Color :type Linear%20Color%20Structure))
  (if (Variables|Default|GetDebug)
    (Class|MordhauUtilityLibrary|PrinttoConsoleandLog Msg)
    (Development|PrintString Msg true true Color 1e+01)))

(fn OnRepCurrentMat
  (Networking|SwitchHasAuthority
    (:Authority
      (Development|PrintString "Point Changed Color" true true "(R=1.000000,G=0.000000,B=0.079762,A=1.000000)"))
    (:Remote
      (Development|PrintString "Point Changed Color" true true "(R=0.000000,G=1.000000,B=0.013482,A=1.000000)")))
  (Rendering|Material|SetMaterial (Variables|Default|GetStaticMesh) 0 (Variables|RepNotify|GetCurrentMat)))

(fn SetPointColor
  (bind _teamcolors (Variables|Color|GetTeamColors))
  (if (or (Utilities|Time|IsTimerActivebyHandle (Variables|Private|GetLifeHandle)) (Variables|HardpointSystem|GetActive))
    (if (and (!= (Variables|RepNotify|GetTeam0PlayersOnPoint) 0) (!= (Variables|RepNotify|GetTeam1PlayersOnPoint) 0))
      (Variables|RepNotify|SetCurrentMat (Variables|Color|GetActive%20Mat) :!label _label)
      (elif (!= (Variables|RepNotify|GetTeam1PlayersOnPoint) 0)
        (Variables|RepNotify|SetCurrentMat (.Value (Utilities|Map|Find _teamcolors "NewEnumerator0")))
        (elif (!= (Variables|RepNotify|GetTeam0PlayersOnPoint) 0)
          (Variables|RepNotify|SetCurrentMat (.Value (Utilities|Map|Find _teamcolors "NewEnumerator1")))
          (else
            (goto _label)))))
    (else
      (Variables|RepNotify|SetCurrentMat (Variables|Color|GetInactive%20Mat)))))

(fn OnRepTeam1PlayersonPoint
  (Update|OnActivePlayersChanged))

(fn OnRepTeam0PlayersonPoint
  (Update|OnActivePlayersChanged))

(fn OnActivePlayersChanged
  (Networking|SwitchHasAuthority
    (:Authority
      (if (== (Variables|RepNotify|GetTeam1PlayersOnPoint) 0)
        (Utilities|Time|PauseTimerbyHandle (Variables|Private|GetAddScoreTeam1Timer))
        (Debug|DebugPrint "Team1 Timer Paused" "(R=0.000000,G=1.000000,B=0.043137,A=1.000000)")
        (elif (== (Variables|RepNotify|GetTeam0PlayersOnPoint) 0)
          (Utilities|Time|PauseTimerbyHandle (Variables|Private|GetAddScoreTeam0Timer))
          (Debug|DebugPrint "Team0 Timer Paused" "(R=0.000000,G=1.000000,B=0.043137,A=1.000000)")))
      (CallFunction|ServerUpdate)
      (CallFunction|ServerUpdateColor))))

(fn CheckPlayersonPoint)

(fn UpdatePointIconData
  (params (Team0%20Count :type Integer) (Team1%20Count :type Integer) (Percentage :type Float%20%28single-precision%29))
  (Networking|CanExecuteCosmeticEvents
    (:True
      (bind _asui_point_icon (Utilities|Casting|CastToUI_PointIcon (UserInterface|GetUserWidgetObject (Variables|Default|GetPointUI))))
      (Rendering|Components|TextRender|SetText (Variables|/Game/Mordhau/Maps/Mordhau-Hardpoint/Assets/BPS/UI_PointIcon.UI_PointIcon_C|GetTeam0 _asui_point_icon) (Utilities|Text|ToText(Integer) Team0%20Count))
      (Rendering|Components|TextRender|SetText (Variables|/Game/Mordhau/Maps/Mordhau-Hardpoint/Assets/BPS/UI_PointIcon.UI_PointIcon_C|GetTeam1 _asui_point_icon) (Utilities|Text|ToText(Integer) Team1%20Count)))))