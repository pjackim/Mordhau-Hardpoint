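; Manager for a Mordhau Hardpoint mode that rotates the active BP_Hardpoint and overrides Team Deathmatch scoring and respawn rules, with fewer overrides for Push.
; The construction script selection-sorts placed hardpoints by Order and recursively resolves the starting point.
; BeginPlay activates it and binds its next-point event, which advances through the array with wraparound.
; UpdateTimer feeds the current point's remaining time to UI_Timer progress bars; widget creation code is unconnected.
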(event Custom|ServerGetNextHardpoint
  (CallFunction|ClientGetNextHardpoint))

(event Custom|ClientGetNextHardpoint
  (CallFunction|GetNextHardpoint)
  (EventDispatchers|BindEventtoGetNewPoint (Variables|Default|GetCurrentHardpoint) (EventDispatchers|CreateEvent :!event Custom|ServerGetNextHardpoint)))

(event Custom|UpdateUI
  ;[1 1 1] Some Shit you don't need to worry about. Does nothing rn
  (CallFunction|UpdateTimer))

(event Custom|ServerUI
  ;[1 1 1] Some Shit you don't need to worry about. Does nothing rn
  (CallFunction|UpdateUI))

(event Custom|Client%20Disable%20All%20Active%20Points
  (for _array_element (Variables|Default|GetHardpoints)
    (if (Utilities|Time|IsValidTimerHandle (Variables|/Game/Mordhau/Maps/Mordhau-Hardpoint/Assets/BPS/BP_Hardpoint.BP_Hardpoint_C|GetLifeHandle _array_element))
      (Default|ServerSetInactive _array_element))))

(event Custom|Server%20Disable%20All%20Active%20Points
  (CallFunction|ClientDisableAllActivePoints))

(event EventBeginPlay
  (CallFunction|EditGameMode)
  (Default|ServerSetActive (Utilities|Array|Get(acopy) (Variables|Default|GetHardpoints) (Variables|Default|GetCurrentIndex)))
  (bind _currenthardpoint (Variables|Default|GetCurrentHardpoint)
    (:then
      (EventDispatchers|BindEventtoGetNewPoint _currenthardpoint (delegate Custom|ServerGetNextHardpoint)))
    (:else)))

(event EventTick
  (params (DeltaSeconds :type Float%20%28single-precision%29)))

(fn ConstructionScript
  (Utilities|Array|Clear (LocalVariables|GettempHardpoints))
  (Utilities|Array|Clear (Variables|Default|GetHardpoints))
  (bind _outactors (Actor|GetAllActorsOfClass "/Game/Mordhau/Maps/Mordhau-Hardpoint/Assets/BPS/BP_Hardpoint.BP_Hardpoint_C"))
  (bind _output_get (LocalVariables|SettempHardpoints _outactors))
  (for (_array_element _array_index) _output_get :!label _label
    (if (== _array_index 0)
      (LocalVariables|SethighestPriority _array_element)
      (elif (> (Variables|/Game/Mordhau/Maps/Mordhau-Hardpoint/Assets/BPS/BP_Hardpoint.BP_Hardpoint_C|GetOrder _array_element) (Variables|/Game/Mordhau/Maps/Mordhau-Hardpoint/Assets/BPS/BP_Hardpoint.BP_Hardpoint_C|GetOrder (LocalVariables|GethighestPriority)))
        (LocalVariables|SethighestPriority _array_element))))
  (if (== (Utilities|Array|Length (LocalVariables|GettempHardpoints)) 0)
    (for _array_element_2 (Variables|Default|GetHardpoints)
      (if (> (Variables|/Game/Mordhau/Maps/Mordhau-Hardpoint/Assets/BPS/BP_Hardpoint.BP_Hardpoint_C|GetOrder _array_element_2) (Variables|Default|GetHighestOrder1))
        (Variables|Default|SetHighestOrder1 (Variables|/Game/Mordhau/Maps/Mordhau-Hardpoint/Assets/BPS/BP_Hardpoint.BP_Hardpoint_C|GetOrder _array_element_2))
        (elif (< (Variables|/Game/Mordhau/Maps/Mordhau-Hardpoint/Assets/BPS/BP_Hardpoint.BP_Hardpoint_C|GetOrder _array_element_2) (Variables|Default|GetLowestOrder1))
          (Variables|Default|SetLowestOrder1 (Variables|/Game/Mordhau/Maps/Mordhau-Hardpoint/Assets/BPS/BP_Hardpoint.BP_Hardpoint_C|GetOrder _array_element_2)))))
    (bind _hardpoint (CallFunction|GetHardpointat (Variables|Default|GetCurrentOrder)))
    (bind _output_get_2 (Variables|Default|SetCurrentHardpoint _hardpoint))
    (Variables|Default|SetCurrentOrder (Variables|/Game/Mordhau/Maps/Mordhau-Hardpoint/Assets/BPS/BP_Hardpoint.BP_Hardpoint_C|GetOrder _output_get_2))
    (Default|ServerSetActive _output_get_2)
    (else
      (Utilities|Array|Insert (Variables|Default|GetHardpoints) (LocalVariables|GethighestPriority))
      (Utilities|Array|RemoveItem (LocalVariables|GettempHardpoints) (LocalVariables|GethighestPriority))
      (goto _label))))

(fn GetNextHardpoint
  (if (>= (+ (Variables|Default|GetCurrentIndex) 1) (Utilities|Array|Length (Variables|Default|GetHardpoints)))
    (Variables|Default|SetCurrentIndex 0)
    (else
      (Math|Integer|IncrementInt (Variables|Default|GetCurrentIndex)
        (:%20%20
          _))))
  (bind _output_get (Variables|Default|SetCurrentHardpoint (Utilities|Array|Get(acopy) (Variables|Default|GetHardpoints) (Variables|Default|GetCurrentIndex))))
  (Default|ServerSetActive _output_get))

(fn GetHardpointat
  (params (Priority :type Integer))
  ;[1 1 1] Lil bit of recursion. If you are new to programming, I would not look at this
  (if (and (<= Priority (Variables|Default|GetHighestOrder1)) (>= Priority (Variables|Default|GetLowestOrder1)))
    (for (_array_element _array_index) (Variables|Default|GetHardpoints)
      (if (== (Variables|/Game/Mordhau/Maps/Mordhau-Hardpoint/Assets/BPS/BP_Hardpoint.BP_Hardpoint_C|GetOrder _array_element) Priority)
        (Variables|Default|SetCurrentIndex _array_index)
        (return _array_element)))
    (bind _hardpoint (CallFunction|GetHardpointat (+ Priority 1)))
    (return _hardpoint)
    (else
      (return (Utilities|Array|Get(acopy) (Variables|Default|GetHardpoints))))))

(fn UpdateTimer
  (bind _currenthardpoint (Variables|Default|GetCurrentHardpoint))
  (Networking|CanExecuteCosmeticEvents
    (:True
      (bind _foundwidgets (Widget|GetAllWidgetsOfClass "/Game/Mordhau/Maps/Mordhau-Hardpoint/Assets/BPS/UI_Timer.UI_Timer_C" false))
      (for _array_element _foundwidgets
        (Progress|SetPercent (Variables|/Game/Mordhau/Maps/Mordhau-Hardpoint/Assets/BPS/UI_Timer.UI_Timer_C|GetProgressBar_33 _array_element) (/ (Utilities|Time|GetTimerRemainingTimebyHandle (Variables|/Game/Mordhau/Maps/Mordhau-Hardpoint/Assets/BPS/BP_Hardpoint.BP_Hardpoint_C|GetLifeHandle _currenthardpoint)) (Variables|/Game/Mordhau/Maps/Mordhau-Hardpoint/Assets/BPS/BP_Hardpoint.BP_Hardpoint_C|GetpointDuration _currenthardpoint)))))))

(fn EditGameMode
  (bind _returnvalue (Game|GetGameMode))
  (bind _hp_killvalue (Variables|Gamemode|GetHP_KillValue))
  (bind _asbp_team_deathmatch_game_mode (Utilities|Casting|CastToBP_TeamDeathmatchGameMode _returnvalue)
    (:then
      (Variables|/Script/Mordhau.MordhauGameMode|SetAssistDamageToCountAsKill _asbp_team_deathmatch_game_mode 50)
      (Variables|/Script/Mordhau.MordhauGameMode|SetKillScoreChange _asbp_team_deathmatch_game_mode _hp_killvalue)
      (Variables|/Script/Mordhau.MordhauGameMode|SetKillTeamScoreChange _asbp_team_deathmatch_game_mode 0.0)
      (Variables|/Game/Mordhau/Blueprints/GameModes/BP_TeamDeathmatchGameMode.BP_TeamDeathmatchGameMode_C|SetTeamScoreToWin _asbp_team_deathmatch_game_mode (Variables|Gamemode|GetHP_ScoreLimit))
      (Variables|/Script/Mordhau.MordhauGameMode|SetbUsesSlowPlayerSpawning _asbp_team_deathmatch_game_mode true)
      (Variables|/Script/Mordhau.MordhauGameMode|SetPlayerRespawnTime _asbp_team_deathmatch_game_mode (Variables|Gamemode|GetHP_RespawnTime))
      (Variables|/Script/Mordhau.MordhauGameMode|SetbPlayersSpawnInWaves _asbp_team_deathmatch_game_mode true)
      (Variables|/Script/Mordhau.MordhauGameMode|SetTeamKillTeamScoreChange _asbp_team_deathmatch_game_mode 0.0)
      (Variables|/Script/Mordhau.MordhauGameMode|SetTeamKillScoreChange _asbp_team_deathmatch_game_mode (Variables|Gamemode|GetHP_TeamKillPen))
      (bind _asbp_team_deathmatch_game_state (Utilities|Casting|CastToBP_TeamDeathmatchGameState (Game|GetGameState)))
      (Variables|/Script/Mordhau.MordhauGameState|SetDefaultWarmupTime _asbp_team_deathmatch_game_state (Variables|Gamemode|GetHP_Warmup)))
    (:CastFailed
      (bind _asbp_push_game_mode (Utilities|Casting|CastToBP_PushGameMode _returnvalue))
      (Variables|/Script/Mordhau.MordhauGameMode|SetKillScoreChange _asbp_push_game_mode _hp_killvalue)
      (Variables|/Script/Mordhau.MordhauGameMode|SetKillTeamScoreChange _asbp_push_game_mode 0.0))))